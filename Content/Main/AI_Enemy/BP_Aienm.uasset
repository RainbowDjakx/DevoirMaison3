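; Melee enemy AI actor that turns toward the player, attacks on proximity and can be damaged until it collapses.
; Entering the face range starts a looping timer that smoothly rotates its yaw toward the player until an overlap ends.
; The attack range triggers a montage gated by DoOnce and a cooldown.
; Player capsule contact arms the damage event, which lowers Life with a delayed reset, simulating mesh physics once Life is depleted.
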(event `self.Face_Range.OnComponentBeginOverlap`
  (params (OverlappedComponent :type "PrimitiveComponent Object Reference") (OtherActor :type "Actor Object Reference") (OtherComp :type "PrimitiveComponent Object Reference") (OtherBodyIndex :type Integer) (bFromSweep :type Boolean) (SweepResult :type "HitResult Structure (by ref)"))
  ;[0.1961 0 0] Look at
  (if (not (`self.IsAttack`))
    (bind _asbp_third_person_character (cast `/Game/Main/Player/BP_ThirdPersonCharacter` OtherActor))
    (set `self.Ref_Character` _asbp_third_person_character)
    (bind _returnvalue (`KismetSystemLibrary.K2_SetTimerDelegate` (delegate `Event_Rotate`) 0.01 true))
    (set `self.FaceAt_Timer` _returnvalue)))

(event `Event_Rotate`
  (bind (_returnvalue_roll _returnvalue_pitch _returnvalue_yaw) (`KismetMathLibrary.BreakRotator` (`KismetMathLibrary.RInterpTo` (`self.K2_GetActorRotation`) (`KismetMathLibrary.FindLookAtRotation` (`self.K2_GetActorLocation`) (`self.K2_GetActorLocation` (`self.Ref_Character`))) (`GameplayStatics.GetWorldDeltaSeconds`) 1.0)))
  ;[0.1961 0 0] Look at
  (`self.K2_SetActorRotation` (`KismetMathLibrary.MakeRotator` 0.0 0.0 _returnvalue_yaw)))

(event `Event_TakeDamage`
  (if (`self.IsTouched`)
    (set `self.CanTakeDamage` false)
    (set `self.IsTouched` false)
    (`KismetSystemLibrary.PrintString` "aouch")
    (`self.Event_DamageAplie`)
    (`KismetSystemLibrary.Delay` 2.0)
    (set `self.CanTakeDamage` true)
    (goto _label :!via `Reset`)))

(event `self.Face_Range.OnComponentEndOverlap`
  (params (OverlappedComponent :type "PrimitiveComponent Object Reference") (OtherActor :type "Actor Object Reference") (OtherComp :type "PrimitiveComponent Object Reference") (OtherBodyIndex :type Integer))
  ;[0.1961 0 0] End Look at
  (`KismetSystemLibrary.K2_ClearAndInvalidateTimerHandle` (`self.FaceAt_Timer`)))

(event `self.CapsuleComponent.OnComponentBeginOverlap`
  (params (OverlappedComponent :type "PrimitiveComponent Object Reference") (OtherActor :type "Actor Object Reference") (OtherComp :type "PrimitiveComponent Object Reference") (OtherBodyIndex :type Integer) (bFromSweep :type Boolean) (SweepResult :type "HitResult Structure (by ref)"))
  (cast `/Game/Main/Player/BP_ThirdPersonCharacter` OtherActor)
  (`/Engine/EditorBlueprintResources/StandardMacros.DoOnce` false :!label _label
    (:`Completed`
      (set `self.IsTouched` true))))

(event `self.Attack_Range.OnComponentBeginOverlap`
  (params (OverlappedComponent :type "PrimitiveComponent Object Reference") (OtherActor :type "Actor Object Reference") (OtherComp :type "PrimitiveComponent Object Reference") (OtherBodyIndex :type Integer) (bFromSweep :type Boolean) (SweepResult :type "HitResult Structure (by ref)"))
  ;[0.1961 0 0] Attack on sight
  (cast `/Game/Main/Player/BP_ThirdPersonCharacter` OtherActor)
  (`KismetSystemLibrary.PrintString` "Human detected" true true (struct :`G` 0.66 :`B` 1.0 :`A` 1.0) 0.1)
  (if (`self.CanAttack`)
    (`self.Event_IaAttack`)))

(event `Event_DamageAplie`
  (if (> (`self.Life`) 0.0)
    (bind _output_get (set `self.Life` (- (`self.Life`) 2.0)))
    (`KismetSystemLibrary.PrintString` (`KismetStringLibrary.Conv_DoubleToString` _output_get))
    (else
      (`PrimitiveComponent.SetSimulatePhysics` (`self.Mesh`) true))))

(event `Event_IaAttack`
  ;[0.2118 0.3059 0.502] HeavyAttack
  (`/Engine/EditorBlueprintResources/StandardMacros.DoOnce` false :!label _label_2
    (:`Completed`
      (set `self.CanAttack` false)
      (set `self.IsAttack` true)
      (`|PlayMontage` (`self.Mesh`) "/Game/Main/Animations/Sequence1/02_Attack/05_Combo_Attack_Wave_05/AM_Ia_attack_front.AM_Ia_attack_front" 0.8
        (:`OnCompleted`
          _)
        (:`OnInterrupted`
          _))
      (set `self.IsAttack` false)
      (`KismetSystemLibrary.Delay` 1.0)
      (set `self.CanAttack` true)
      (goto _label_2 :!via `Reset`))))

(fn `UserConstructionScript`)